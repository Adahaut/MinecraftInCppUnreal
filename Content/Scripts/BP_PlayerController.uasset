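; Player controller that lets the player break and place blocks in a chunked voxel world.
; Both mouse buttons line trace from the camera up to BlockDistance and convert the hit to a chunk-local block position on BP_GreedyChunk.
; Left click sets the hit voxel to Air through ModifyVoxel.
; Right click places Stone in the adjacent cell along the hit normal, gated by distance checks against the player capsule's bounds.
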(event `InputAction|RightMouseButton`
  (params (Key :type "Key Structure"))
  (:`Pressed`
    (bind (_returnvalue _outhit) (`self.Raycast`))
    (if _returnvalue
      (bind _asbp_player_character (cast `/Game/Scripts/BP_PlayerCharacter` (`GameplayStatics.GetPlayerCharacter` 0)))
      (bind (_bblockinghit _binitialoverlap _time _distance _location _impactpoint _normal _impactnormal _physmat _hitactor) (`GameplayStatics.BreakHitResult` _outhit))
      (bind _asbp_greedy_chunk (cast `/Game/Scripts/BP_GreedyChunk` _hitactor))
      (bind _returnvalue_2 (- _location _normal))
      (bind (_origin _boxextent) (`KismetSystemLibrary.GetComponentBounds` (`Character.CapsuleComponent` _asbp_player_character)))
      (if (and (> (`KismetMathLibrary.Vector_Distance` _returnvalue_2 _origin) 150.0) (> (`KismetMathLibrary.Vector_Distance` _returnvalue_2 _boxextent) 150.0))
        (`GreedyChunk.ModifyVoxel` _asbp_greedy_chunk (`KismetMathLibrary.FTruncVector` (+ (`VoxelFunctionLibrary.WorldToLocalBlockPosition` _returnvalue_2 (`self.ChunkSize`)) _normal)) "Stone")))))

(event `InputAction|LeftMouseButton`
  (params (Key :type "Key Structure"))
  (:`Pressed`
    (bind (_returnvalue _outhit) (`self.Raycast`))
    (if _returnvalue
      (bind (_bblockinghit _binitialoverlap _time _distance _location _impactpoint _normal _impactnormal _physmat _hitactor) (`GameplayStatics.BreakHitResult` _outhit))
      (bind _asbp_greedy_chunk (cast `/Game/Scripts/BP_GreedyChunk` _hitactor))
      (`GreedyChunk.ModifyVoxel` _asbp_greedy_chunk (`VoxelFunctionLibrary.WorldToLocalBlockPosition` (- _location _normal) (`self.ChunkSize`)) "Air"))))

(fn `Raycast`
  (returns (ReturnValue :type Boolean) (OutHit :type "HitResult Structure"))
  (bind _playercameramanager (`self.PlayerCameraManager`))
  (bind _returnvalue (`PlayerCameraManager.GetCameraLocation` _playercameramanager))
  (bind (_outhit _returnvalue_2) (`KismetSystemLibrary.LineTraceSingle` :`Start` _returnvalue :`End` (+ _returnvalue (* (`KismetMathLibrary.GetForwardVector` (`PlayerCameraManager.GetCameraRotation` _playercameramanager)) (`self.BlockDistance`))) :`TraceChannel` "TraceTypeQuery1" :`DrawTime` 1.0))
  (return _returnvalue_2 _outhit))

(fn `UserConstructionScript`)