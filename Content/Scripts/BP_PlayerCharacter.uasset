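; Player character Blueprint that handles jumping, movement and mouse look.
; Jump sets the movement component's jump Z velocity from JumpForce before jumping.
; MoveX and MoveY share one AddInputVector call, combining axis-value vectors multiplied component-wise by the actor's right and forward vectors.
; Mouse axes drive controller yaw and pitch scaled by MouseSensitivity, while MoveZ is unimplemented.
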(event `InputAction|Jump`
  (params (Key :type "Key Structure"))
  (:`Pressed`
    (set `CharacterMovementComponent.JumpZVelocity` (`self.JumpForce`) (`self.CharacterMovement`))
    (`self.Jump`)))

(event `InputAxis|MoveZ`
  (params (AxisValue :type "Float (single-precision)")))

(event `InputAxis|MoveY`
  (params (AxisValue :type "Float (single-precision)"))
  (`PawnMovementComponent.AddInputVector` (`self.CharacterMovement`) (+ (* (`KismetMathLibrary.MakeVector` AxisValue AxisValue) (`self.GetActorRightVector`)) (* (`KismetMathLibrary.MakeVector` (stale `InputAxis|MoveX` AxisValue) (stale `InputAxis|MoveX` AxisValue)) (`self.GetActorForwardVector`))) false :!label _label))

(event `InputAxis|MoveX`
  (params (AxisValue :type "Float (single-precision)"))
  (goto _label))

(event `InputAxis|MouseY`
  (params (AxisValue :type "Float (single-precision)"))
  (`self.AddControllerPitchInput` (* AxisValue (`self.MouseSensitivity`))))

(event `InputAxis|MouseX`
  (params (AxisValue :type "Float (single-precision)"))
  (`self.AddControllerYawInput` (* AxisValue (`self.MouseSensitivity`))))

(fn `UserConstructionScript`)